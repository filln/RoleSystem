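; BP_RoleTestWidgetManager manages the role system's test UI, the WBP_RoleTestBasicParameters widget.
; It creates and stores that widget on BeginPlay.
; A toggle function checks the widget's visibility and delegates showing or hiding it to the core classes manager reached through RoleSystemRootComponent.
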(event `self.ReceiveBeginPlay`
  (bind _returnvalue (`|CreateWidget` "/Game/RoleSystem/TestSystem/Widgets/WBP_RoleTestBasicParameters.WBP_RoleTestBasicParameters_C"))
  (set `self.WBP_RoleTestMain` _returnvalue))

(fn `ShowOrHideWBP_RoleTestMain`
  (bind _wbp_roletestmain (`self.WBP_RoleTestMain`))
  (if (`Widget.IsVisible` _wbp_roletestmain)
    (`/Game/RoleSystem/Blueprints/BP_RoleSystemCoreClassesManager.ShowOrHideWidget` (`/Game/RoleSystem/Blueprints/RoleSystemRootComponent.BP_RoleSystemCoreClassesManager` (`self.RoleSystemRootComponent`)) false _wbp_roletestmain 0)
    (else
      (`/Game/RoleSystem/Blueprints/BP_RoleSystemCoreClassesManager.ShowOrHideWidget` (`/Game/RoleSystem/Blueprints/RoleSystemRootComponent.BP_RoleSystemCoreClassesManager` (`self.RoleSystemRootComponent`)) true _wbp_roletestmain 0))))

(fn `UserConstructionScript`)