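; Manager for the role system's core classes that caches the HUD and player controller and centralizes widget, input mode and pause control.
; On BeginPlay it stores both cast and uncast references, the latter to ease porting between projects, then calls empty HUD and controller setup functions.
; Pausing toggles an optional widget and applies the given input mode with matching cursor visibility.
; ChangeInputMode switches between game-only and game-and-UI input.
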(event `self.ReceiveBeginPlay`
  (`self.GetReferencesToCoreObjects`)
  (`self.BeginPlayHUD`)
  (`self.BeginPlayPlayerController`))

(fn `BeginPlayHUD`)

(fn `BeginPlayPlayerController`)

(fn `ChangeInputMode`
  (if (`|EnumEquality` (`self.InputMode`) "NewEnumerator1")
    (bind _output_get (set `self.InputMode` "NewEnumerator2"))
    (`self.SetInputMode` _output_get)
    (else
      (bind _output_get_2 (set `self.InputMode` "NewEnumerator1"))
      (`self.SetInputMode` _output_get_2))))

(fn `GetReferencesToCoreObjects`
  (`|ExecutionSequence`
    (:`then_0`
      ;[0 0.2031 1] Взять ссылку на ХУД.
      (bind (_asbp_hudrole_system _iscastsuccess_) (`/Game/RoleSystem/Blueprints/CoreClasses/BPFL_ReferenceAggregator.GetHUD`))
      (if _iscastsuccess_
        (set `self.BP_HUDRoleSystem` _asbp_hudrole_system)
        ;;[0 1 0.5547] Возможно где-то хватит нескастованной ссылки. Поможет избежать лишних исправлений при переносе в другой проект.
        (set `self.HUD` (`PlayerController.GetHUD` (`GameplayStatics.GetPlayerController` 0)))))
    (:`then_1`
      ;[1 0.3281 0] Взять ссылку на Контроллер.
      (bind (_asbp_player_controller_role_system _iscastsuccess__2) (`/Game/RoleSystem/Blueprints/CoreClasses/BPFL_ReferenceAggregator.GetPlayerController`))
      (if _iscastsuccess__2
        (set `self.BP_PlayerControllerRoleSystem` _asbp_player_controller_role_system)
        ;;[1 0 0.3281] Возможно где-то хватит нескастованной ссылки. Поможет избежать лишних исправлений при переносе в другой проект.
        (set `self.PlayerController` (`GameplayStatics.GetPlayerController` 0))))))

(fn `PauseOrUnpauseGame`
  (params (`isPause?` :type Boolean) (_OnWidgetIfPause :type "UserWidget Object Reference") (ZOrderOnWidget :type Integer) (_OffWidgetIfUnpause :type "UserWidget Object Reference") (InputModePause :type "/Game/RoleSystem/Enums/EInputModeRoleSystem Enum" :default "NewEnumerator0") (InputModeUnPause :type "/Game/RoleSystem/Enums/EInputModeRoleSystem Enum" :default "NewEnumerator0"))
  (if `isPause?`
    (if (`GameplayStatics.IsGamePaused`)
      (return)
      (else
        (`GameplayStatics.SetGamePaused` true)
        (if (`KismetSystemLibrary.IsValid` _OnWidgetIfPause)
          (`self.ShowOrHideWidget` true _OnWidgetIfPause ZOrderOnWidget))
        (`self.SetInputMode` InputModePause _OnWidgetIfPause)
        (return)))
    (elif (`GameplayStatics.IsGamePaused`)
      (`GameplayStatics.SetGamePaused` false)
      (`self.SetInputMode` InputModeUnPause)
      (if (`KismetSystemLibrary.IsValid` _OffWidgetIfUnpause)
        (`self.ShowOrHideWidget` false _OffWidgetIfUnpause))
      (return)
      (else
        (return)))))

(fn `SetInputMode`
  (params (InputMode :type "/Game/RoleSystem/Enums/EInputModeRoleSystem Enum" :default "NewEnumerator0") (InWidgetToFocus :type "Widget Object Reference"))
  (bind _playercontroller (`self.PlayerController`))
  (if (`|EnumEquality` InputMode "NewEnumerator0")
    (set `PlayerController.bShowMouseCursor` true _playercontroller)
    (`WidgetBlueprintLibrary.SetInputMode_UIOnlyEx` _playercontroller InWidgetToFocus)
    (elif (`|EnumEquality` InputMode "NewEnumerator1")
      (set `PlayerController.bShowMouseCursor` false _playercontroller)
      (`WidgetBlueprintLibrary.SetInputMode_GameOnly` _playercontroller)
      (elif (`|EnumEquality` InputMode "NewEnumerator2")
        (set `PlayerController.bShowMouseCursor` true _playercontroller)
        (`WidgetBlueprintLibrary.SetInputMode_GameAndUIEx` _playercontroller InWidgetToFocus "DoNotLock" false)
        (else
          (return)))))
  (return))

(fn `ShowOrHideWidget`
  (params (`isShow?` :type Boolean) (UserWidgetRef :type "UserWidget Object Reference") (ZOrder :type Integer))
  (if `isShow?`
    (if (`Widget.IsVisible` UserWidgetRef)
      (return)
      (else
        (`UserWidget.AddToViewport` UserWidgetRef ZOrder)))
    (elif (`Widget.IsVisible` UserWidgetRef)
      (`Widget.RemoveFromParent` UserWidgetRef)
      (else
        (return))))
  (return))

(fn `UserConstructionScript`)