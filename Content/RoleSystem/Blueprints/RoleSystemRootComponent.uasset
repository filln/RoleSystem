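; Root component of the RPG role system that spawns and holds every actor the system uses.
; On BeginPlay it spawns the class, widget and item managers, then separate actors for age stages, attributes, skills, perks, resistances, stamina, wounds and other parameters.
; It stores a reference to each and sets itself as their RoleSystemRootComponent, acting as the shared hub.
; A second pass spawns the role-test widget manager the same way.
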(event `self.ReceiveBeginPlay`
  (`self.SpawnAllRoleSystemActors`)
  (`self.SpawnAllRoleTestSystemActors`))

(fn `SpawnAllRoleSystemActors`
  (`|ExecutionSequence`
    (:`then_0`
      (bind _returnvalue (`|SpawnActorFromClass` "/Game/RoleSystem/Blueprints/AgeStages/BP_AgeStages.BP_AgeStages_C" (`self.SpawnTransform`) "AlwaysSpawn" "OverrideRootScale" null null))
      (bind _output_get (set `self.BP_AgeStages` _returnvalue))
      (set `/Game/RoleSystem/Blueprints/BP_RoleSystemParent.RoleSystemRootComponent` self _output_get)
      ;[0.1719 1 0] Спавнить BP_CoreClassesManager
      (bind _returnvalue_2 (`|SpawnActorFromClass` "/Game/RoleSystem/Blueprints/BP_RoleSystemCoreClassesManager.BP_RoleSystemCoreClassesManager_C" (`self.SpawnTransform`) "AlwaysSpawn" "OverrideRootScale" null null))
      (bind _output_get_2 (set `self.BP_RoleSystemCoreClassesManager` _returnvalue_2))
      (set `/Game/RoleSystem/Blueprints/BP_RoleSystemParent.RoleSystemRootComponent` self _output_get_2)
      ;[0.9219 1 0] Спавнить BP_RoleSystemWidgetManager
      (bind _returnvalue_3 (`|SpawnActorFromClass` "/Game/RoleSystem/Blueprints/BP_RoleSystemWidgetManager.BP_RoleSystemWidgetManager_C" (`self.SpawnTransform`) "AlwaysSpawn" "OverrideRootScale" null null))
      (bind _output_get_3 (set `self.BP_RoleSystemWidgetManager` _returnvalue_3))
      (set `/Game/RoleSystem/Blueprints/BP_RoleSystemParent.RoleSystemRootComponent` self _output_get_3)
      ;[0.07812 0 1] Спавнить BP_RoleSystemItemsManager
      (bind _returnvalue_4 (`|SpawnActorFromClass` "/Game/RoleSystem/Blueprints/BP_RoleSystemItemsManager.BP_RoleSystemItemsManager_C" (`self.SpawnTransform`) "AlwaysSpawn" "OverrideRootScale" null null))
      (bind _output_get_4 (set `self.BP_RoleSystemItemsManager` _returnvalue_4))
      (set `/Game/RoleSystem/Blueprints/BP_RoleSystemParent.RoleSystemRootComponent` self _output_get_4))
    (:`then_1`
      (`self.SpawnBasicParameters`))
    (:`then_2`
      (`self.SpawnBasicSkills`))
    (:`then_3`
      (bind _returnvalue_5 (`|SpawnActorFromClass` "/Game/RoleSystem/Blueprints/OtherParameters/BP_OtherParameters.BP_OtherParameters_C" (`self.SpawnTransform`) "AlwaysSpawn" "OverrideRootScale" null null))
      (bind _output_get_5 (set `self.BP_OtherParameters` _returnvalue_5))
      (set `/Game/RoleSystem/Blueprints/BP_RoleSystemParent.RoleSystemRootComponent` self _output_get_5))
    (:`then_4`
      (`self.SpawnPerks`))
    (:`then_5`
      (bind _returnvalue_6 (`|SpawnActorFromClass` "/Game/RoleSystem/Blueprints/Resistances/BP_Resistances.BP_Resistances_C" (`self.SpawnTransform`) "AlwaysSpawn" "OverrideRootScale" null null))
      (bind _output_get_6 (set `self.BP_Resistances` _returnvalue_6))
      (set `/Game/RoleSystem/Blueprints/BP_RoleSystemParent.RoleSystemRootComponent` self _output_get_6))
    (:`then_6`
      (bind _returnvalue_7 (`|SpawnActorFromClass` "/Game/RoleSystem/Blueprints/SecondaryParameters/BP_Stamina.BP_Stamina_C" (`self.SpawnTransform`) "AlwaysSpawn" "OverrideRootScale" null null))
      (bind _output_get_7 (set `self.BP_Stamina` _returnvalue_7))
      (set `/Game/RoleSystem/Blueprints/BP_RoleSystemParent.RoleSystemRootComponent` self _output_get_7))
    (:`then_7`
      (bind _returnvalue_8 (`|SpawnActorFromClass` "/Game/RoleSystem/Blueprints/Wounds/BP_Wounds.BP_Wounds_C" (`self.SpawnTransform`) "AlwaysSpawn" "OverrideRootScale" null null))
      (bind _output_get_8 (set `self.BP_Wounds` _returnvalue_8))
      (set `/Game/RoleSystem/Blueprints/BP_RoleSystemParent.RoleSystemRootComponent` self _output_get_8))))

(fn `SpawnAllRoleTestSystemActors`
  ;[0.9688 0 1] Спавнить BP_RoleTestWidgetManager
  (bind _returnvalue (`|SpawnActorFromClass` "/Game/RoleSystem/TestSystem/Blueprints/BP_RoleTestWidgetManager.BP_RoleTestWidgetManager_C" (`self.SpawnTransform`) "AlwaysSpawn" "OverrideRootScale" null null))
  (bind _output_get (set `self.BP_RoleTestWidgetManager` _returnvalue))
  (set `/Game/RoleSystem/Blueprints/BP_RoleSystemParent.RoleSystemRootComponent` self _output_get))

(fn `SpawnBasicParameters`
  (`|ExecutionSequence`
    (:`then_0`
      ;[1 0 0.9844] Физический блок
      (bind _returnvalue (`|SpawnActorFromClass` "/Game/RoleSystem/Blueprints/BasicParameters/PhysicalBlock/BP_Strength.BP_Strength_C" (`self.SpawnTransform`) "AlwaysSpawn" "OverrideRootScale" null null))
      (bind _output_get (set `self.BP_Strength` _returnvalue))
      (set `/Game/RoleSystem/Blueprints/BP_RoleSystemParent.RoleSystemRootComponent` self _output_get)
      (bind _returnvalue_2 (`|SpawnActorFromClass` "/Game/RoleSystem/Blueprints/BasicParameters/PhysicalBlock/BP_Dexterity.BP_Dexterity_C" (`self.SpawnTransform`) "AlwaysSpawn" "OverrideRootScale" null null))
      (bind _output_get_2 (set `self.BP_Dexterity` _returnvalue_2))
      (set `/Game/RoleSystem/Blueprints/BP_RoleSystemParent.RoleSystemRootComponent` self _output_get_2)
      (bind _returnvalue_3 (`|SpawnActorFromClass` "/Game/RoleSystem/Blueprints/BasicParameters/PhysicalBlock/BP_Endurance.BP_Endurance_C" (`self.SpawnTransform`) "AlwaysSpawn" "OverrideRootScale" null null))
      (bind _output_get_3 (set `self.BP_Endurance` _returnvalue_3))
      (set `/Game/RoleSystem/Blueprints/BP_RoleSystemParent.RoleSystemRootComponent` self _output_get_3)
      (bind _returnvalue_4 (`|SpawnActorFromClass` "/Game/RoleSystem/Blueprints/BasicParameters/PhysicalBlock/BP_Body.BP_Body_C" (`self.SpawnTransform`) "AlwaysSpawn" "OverrideRootScale" null null))
      (bind _output_get_4 (set `self.BP_Body` _returnvalue_4))
      (set `/Game/RoleSystem/Blueprints/BP_RoleSystemParent.RoleSystemRootComponent` self _output_get_4))))

(fn `SpawnBasicSkills`
  (`|ExecutionSequence`
    (:`then_0`
      (bind _returnvalue (`|SpawnActorFromClass` "/Game/RoleSystem/Blueprints/BasicSkills/BP_Acrobatics.BP_Acrobatics_C" (`self.SpawnTransform`) "AlwaysSpawn" "OverrideRootScale" null null))
      (bind _output_get (set `self.BP_Acrobatics` _returnvalue))
      (set `/Game/RoleSystem/Blueprints/BP_RoleSystemParent.RoleSystemRootComponent` self _output_get)
      (bind _returnvalue_2 (`|SpawnActorFromClass` "/Game/RoleSystem/Blueprints/BasicSkills/BP_Adventurer.BP_Adventurer_C" (`self.SpawnTransform`) "AlwaysSpawn" "OverrideRootScale" null null))
      (bind _output_get_2 (set `self.BP_Adventurer` _returnvalue_2))
      (set `/Game/RoleSystem/Blueprints/BP_RoleSystemParent.RoleSystemRootComponent` self _output_get_2)
      (bind _returnvalue_3 (`|SpawnActorFromClass` "/Game/RoleSystem/Blueprints/BasicSkills/BP_Athletics.BP_Athletics_C" (`self.SpawnTransform`) "AlwaysSpawn" "OverrideRootScale" null null))
      (bind _output_get_3 (set `self.BP_Athletics` _returnvalue_3))
      (set `/Game/RoleSystem/Blueprints/BP_RoleSystemParent.RoleSystemRootComponent` self _output_get_3)
      (bind _returnvalue_4 (`|SpawnActorFromClass` "/Game/RoleSystem/Blueprints/BasicSkills/BP_Diplomat.BP_Diplomat_C" (`self.SpawnTransform`) "AlwaysSpawn" "OverrideRootScale" null null))
      (bind _output_get_4 (set `self.BP_Diplomat` _returnvalue_4))
      (set `/Game/RoleSystem/Blueprints/BP_RoleSystemParent.RoleSystemRootComponent` self _output_get_4))
    (:`then_1`
      (bind _returnvalue_5 (`|SpawnActorFromClass` "/Game/RoleSystem/Blueprints/BasicSkills/BP_Gunsmith.BP_Gunsmith_C" (`self.SpawnTransform`) "AlwaysSpawn" "OverrideRootScale" null null))
      (bind _output_get_5 (set `self.BP_Gunsmith` _returnvalue_5))
      (set `/Game/RoleSystem/Blueprints/BP_RoleSystemParent.RoleSystemRootComponent` self _output_get_5)
      (bind _returnvalue_6 (`|SpawnActorFromClass` "/Game/RoleSystem/Blueprints/BasicSkills/BP_Medic.BP_Medic_C" (`self.SpawnTransform`) "AlwaysSpawn" "OverrideRootScale" null null))
      (bind _output_get_6 (set `self.BP_Medic` _returnvalue_6))
      (set `/Game/RoleSystem/Blueprints/BP_RoleSystemParent.RoleSystemRootComponent` self _output_get_6)
      (bind _returnvalue_7 (`|SpawnActorFromClass` "/Game/RoleSystem/Blueprints/BasicSkills/BP_Psyonic.BP_Psyonic_C" (`self.SpawnTransform`) "AlwaysSpawn" "OverrideRootScale" null null))
      (bind _output_get_7 (set `self.BP_Psyonic` _returnvalue_7))
      (set `/Game/RoleSystem/Blueprints/BP_RoleSystemParent.RoleSystemRootComponent` self _output_get_7)
      (bind _returnvalue_8 (`|SpawnActorFromClass` "/Game/RoleSystem/Blueprints/BasicSkills/BP_Researcher.BP_Researcher_C" (`self.SpawnTransform`) "AlwaysSpawn" "OverrideRootScale" null null))
      (bind _output_get_8 (set `self.BP_Researcher` _returnvalue_8))
      (set `/Game/RoleSystem/Blueprints/BP_RoleSystemParent.RoleSystemRootComponent` self _output_get_8))
    (:`then_2`
      (bind _returnvalue_9 (`|SpawnActorFromClass` "/Game/RoleSystem/Blueprints/BasicSkills/BP_Technician.BP_Technician_C" (`self.SpawnTransform`) "AlwaysSpawn" "OverrideRootScale" null null))
      (bind _output_get_9 (set `self.BP_Technician` _returnvalue_9))
      (set `/Game/RoleSystem/Blueprints/BP_RoleSystemParent.RoleSystemRootComponent` self _output_get_9)
      (bind _returnvalue_10 (`|SpawnActorFromClass` "/Game/RoleSystem/Blueprints/BasicSkills/BP_Warrior.BP_Warrior_C" (`self.SpawnTransform`) "AlwaysSpawn" "OverrideRootScale" null null))
      (bind _output_get_10 (set `self.BP_Warrior` _returnvalue_10))
      (set `/Game/RoleSystem/Blueprints/BP_RoleSystemParent.RoleSystemRootComponent` self _output_get_10))))

(fn `SpawnPerks`
  (`|ExecutionSequence`
    (:`then_0`
      (bind _returnvalue (`|SpawnActorFromClass` "/Game/RoleSystem/Blueprints/Perks/BP_OurProudVaryagDoesNotSurrenderToTheEnemy.BP_OurProudVaryagDoesNotSurrenderToTheEnemy_C" (`self.SpawnTransform`) "AlwaysSpawn" "OverrideRootScale" null null))
      (bind _output_get (set `self.BP_OurProudVaryagDoesNotSurrenderToTheEnemy` _returnvalue))
      (set `/Game/RoleSystem/Blueprints/BP_RoleSystemParent.RoleSystemRootComponent` self _output_get)
      (bind _returnvalue_2 (`|SpawnActorFromClass` "/Game/RoleSystem/Blueprints/Perks/Acrobatics/BP_DeadSilence.BP_DeadSilence_C" (`self.SpawnTransform`) "AlwaysSpawn" "OverrideRootScale" null null))
      (bind _output_get_2 (set `self.BP_DeadSilence` _returnvalue_2))
      (set `/Game/RoleSystem/Blueprints/BP_RoleSystemParent.RoleSystemRootComponent` self _output_get_2)
      (bind _returnvalue_3 (`|SpawnActorFromClass` "/Game/RoleSystem/Blueprints/Perks/Acrobatics/BP_Lemur.BP_Lemur_C" (`self.SpawnTransform`) "AlwaysSpawn" "OverrideRootScale" null null))
      (bind _output_get_3 (set `self.BP_Lemur` _returnvalue_3))
      (set `/Game/RoleSystem/Blueprints/BP_RoleSystemParent.RoleSystemRootComponent` self _output_get_3)
      (bind _returnvalue_4 (`|SpawnActorFromClass` "/Game/RoleSystem/Blueprints/Perks/Adventurer/BP_PlunderEverything.BP_PlunderEverything_C" (`self.SpawnTransform`) "AlwaysSpawn" "OverrideRootScale" null null))
      (bind _output_get_4 (set `self.BP_PlunderEverything` _returnvalue_4))
      (set `/Game/RoleSystem/Blueprints/BP_RoleSystemParent.RoleSystemRootComponent` self _output_get_4))
    (:`then_1`
      (bind _returnvalue_5 (`|SpawnActorFromClass` "/Game/RoleSystem/Blueprints/Perks/Adventurer/BP_PremiumCamouflage.BP_PremiumCamouflage_C" (`self.SpawnTransform`) "AlwaysSpawn" "OverrideRootScale" null null))
      (bind _output_get_5 (set `self.BP_PremiumCamouflage` _returnvalue_5))
      (set `/Game/RoleSystem/Blueprints/BP_RoleSystemParent.RoleSystemRootComponent` self _output_get_5)
      (bind _returnvalue_6 (`|SpawnActorFromClass` "/Game/RoleSystem/Blueprints/Perks/Athletics/BP_Mule.BP_Mule_C" (`self.SpawnTransform`) "AlwaysSpawn" "OverrideRootScale" null null))
      (bind _output_get_6 (set `self.BP_Mule` _returnvalue_6))
      (set `/Game/RoleSystem/Blueprints/BP_RoleSystemParent.RoleSystemRootComponent` self _output_get_6)
      (bind _returnvalue_7 (`|SpawnActorFromClass` "/Game/RoleSystem/Blueprints/Perks/Diplomat/BP_Grilling.BP_Grilling_C" (`self.SpawnTransform`) "AlwaysSpawn" "OverrideRootScale" null null))
      (bind _output_get_7 (set `self.BP_Grilling` _returnvalue_7))
      (set `/Game/RoleSystem/Blueprints/BP_RoleSystemParent.RoleSystemRootComponent` self _output_get_7)
      (bind _returnvalue_8 (`|SpawnActorFromClass` "/Game/RoleSystem/Blueprints/Perks/Diplomat/BP_IfIDidntSingASong.BP_IfIDidntSingASong_C" (`self.SpawnTransform`) "AlwaysSpawn" "OverrideRootScale" null null))
      (bind _output_get_8 (set `self.BP_IfIDidntSingASong` _returnvalue_8))
      (set `/Game/RoleSystem/Blueprints/BP_RoleSystemParent.RoleSystemRootComponent` self _output_get_8))
    (:`then_2`
      (bind _returnvalue_9 (`|SpawnActorFromClass` "/Game/RoleSystem/Blueprints/Perks/Gunsmith/BP_Feather.BP_Feather_C" (`self.SpawnTransform`) "AlwaysSpawn" "OverrideRootScale" null null))
      (bind _output_get_9 (set `self.BP_Feather` _returnvalue_9))
      (set `/Game/RoleSystem/Blueprints/BP_RoleSystemParent.RoleSystemRootComponent` self _output_get_9)
      (bind _returnvalue_10 (`|SpawnActorFromClass` "/Game/RoleSystem/Blueprints/Perks/Gunsmith/BP_IHaveTwoHands.BP_IHaveTwoHands_C" (`self.SpawnTransform`) "AlwaysSpawn" "OverrideRootScale" null null))
      (bind _output_get_10 (set `self.BP_IHaveTwoHands` _returnvalue_10))
      (set `/Game/RoleSystem/Blueprints/BP_RoleSystemParent.RoleSystemRootComponent` self _output_get_10)
      (bind _returnvalue_11 (`|SpawnActorFromClass` "/Game/RoleSystem/Blueprints/Perks/Medic/BP_FirstAidKit.BP_FirstAidKit_C" (`self.SpawnTransform`) "AlwaysSpawn" "OverrideRootScale" null null))
      (bind _output_get_11 (set `self.BP_FirstAidKit` _returnvalue_11))
      (set `/Game/RoleSystem/Blueprints/BP_RoleSystemParent.RoleSystemRootComponent` self _output_get_11)
      (bind _returnvalue_12 (`|SpawnActorFromClass` "/Game/RoleSystem/Blueprints/Perks/Medic/BP_TheresASmallGapBetweenTheFirstAndSecond.BP_TheresASmallGapBetweenTheFirstAndSecond_C" (`self.SpawnTransform`) "AlwaysSpawn" "OverrideRootScale" null null))
      (bind _output_get_12 (set `self.BP_TheresASmallGapBetweenTheFirstAndSecond` _returnvalue_12))
      (set `/Game/RoleSystem/Blueprints/BP_RoleSystemParent.RoleSystemRootComponent` self _output_get_12))
    (:`then_3`
      (bind _returnvalue_13 (`|SpawnActorFromClass` "/Game/RoleSystem/Blueprints/Perks/Researcher/BP_PhDInEngineering.BP_PhDInEngineering_C" (`self.SpawnTransform`) "AlwaysSpawn" "OverrideRootScale" null null))
      (bind _output_get_13 (set `self.BP_PhDInEngineering` _returnvalue_13))
      (set `/Game/RoleSystem/Blueprints/BP_RoleSystemParent.RoleSystemRootComponent` self _output_get_13)
      (bind _returnvalue_14 (`|SpawnActorFromClass` "/Game/RoleSystem/Blueprints/Perks/Researcher/BP_RadioAmateur.BP_RadioAmateur_C" (`self.SpawnTransform`) "AlwaysSpawn" "OverrideRootScale" null null))
      (bind _output_get_14 (set `self.BP_RadioAmateur` _returnvalue_14))
      (set `/Game/RoleSystem/Blueprints/BP_RoleSystemParent.RoleSystemRootComponent` self _output_get_14)
      (bind _returnvalue_15 (`|SpawnActorFromClass` "/Game/RoleSystem/Blueprints/Perks/Technician/BP_ISeeYou.BP_ISeeYou_C" (`self.SpawnTransform`) "AlwaysSpawn" "OverrideRootScale" null null))
      (bind _output_get_15 (set `self.BP_ISeeYou` _returnvalue_15))
      (set `/Game/RoleSystem/Blueprints/BP_RoleSystemParent.RoleSystemRootComponent` self _output_get_15)
      (bind _returnvalue_16 (`|SpawnActorFromClass` "/Game/RoleSystem/Blueprints/Perks/Technician/BP_WhereProgressHasBeenMade.BP_WhereProgressHasBeenMade_C" (`self.SpawnTransform`) "AlwaysSpawn" "OverrideRootScale" null null))
      (bind _output_get_16 (set `self.BP_WhereProgressHasBeenMade` _returnvalue_16))
      (set `/Game/RoleSystem/Blueprints/BP_RoleSystemParent.RoleSystemRootComponent` self _output_get_16))
    (:`then_4`
      (bind _returnvalue_17 (`|SpawnActorFromClass` "/Game/RoleSystem/Blueprints/Perks/Warrior/BP_KickDown.BP_KickDown_C" (`self.SpawnTransform`) "AlwaysSpawn" "OverrideRootScale" null null))
      (bind _output_get_17 (set `self.BP_KickDown` _returnvalue_17))
      (set `/Game/RoleSystem/Blueprints/BP_RoleSystemParent.RoleSystemRootComponent` self _output_get_17)
      (bind _returnvalue_18 (`|SpawnActorFromClass` "/Game/RoleSystem/Blueprints/Perks/Warrior/BP_MapMaker.BP_MapMaker_C" (`self.SpawnTransform`) "AlwaysSpawn" "OverrideRootScale" null null))
      (bind _output_get_18 (set `self.BP_MapMaker` _returnvalue_18))
      (set `/Game/RoleSystem/Blueprints/BP_RoleSystemParent.RoleSystemRootComponent` self _output_get_18))))