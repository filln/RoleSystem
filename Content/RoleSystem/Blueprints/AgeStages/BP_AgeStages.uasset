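; BP_AgeStages handles a character's age stage in the role system and derives the parameter limits for that stage.
; The lower limit scales the combined parameter count of the Physical, Intellectual, Personality and Psyonical blocks by stage and a coefficient.
; The upper limit adds a proportional margin, and the delta between limits drives a linear falloff in parameter gain per step.
; IncreaseStage advances the age enum, clamped to a maximum stage.
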(event `self.ReceiveBeginPlay`
  (`parent.ReceiveBeginPlay`))

(fn `CalcDeltaLimitParameters`
  (params (_LowerLimitParameters :type Integer) (_UpperLimitParameters :type Integer))
  (returns (DeltaLimitParameters :type Integer))
  (return (- _UpperLimitParameters _LowerLimitParameters)))

(fn `CalcGradientIncrease`
  (params (CurrentStep :type Integer) (_DeltaLimitParameters :type "Float (double-precision)"))
  (returns (GradientIncrease :type "Float (double-precision)"))
  (return (- 1.0 (* (`KismetMathLibrary.Conv_IntToDouble` CurrentStep) (/ 1.0 _DeltaLimitParameters)))))

(fn `CalcLowerLimitParameters`
  (params (CoeffAgeStage :type "Float (double-precision)"))
  (returns (LowerLimitParameters :type Integer))
  (return (`KismetMathLibrary.Round` (* (* (+ (`/Game/RoleSystem/Blueprints/BasicParameters/BP_BasicParametersParent.QuantityParametersInBlock` (`/Game/RoleSystem/Blueprints/RoleSystemRootComponent.BP_PhysicalBlock` (`self.RoleSystemRootComponent`))) (`/Game/RoleSystem/Blueprints/BasicParameters/BP_BasicParametersParent.QuantityParametersInBlock` (`/Game/RoleSystem/Blueprints/RoleSystemRootComponent.BP_IntellectualBlock` (`self.RoleSystemRootComponent`))) (`/Game/RoleSystem/Blueprints/BasicParameters/BP_BasicParametersParent.QuantityParametersInBlock` (`/Game/RoleSystem/Blueprints/RoleSystemRootComponent.BP_PersonalityBlock` (`self.RoleSystemRootComponent`))) (`/Game/RoleSystem/Blueprints/BasicParameters/BP_BasicParametersParent.QuantityParametersInBlock` (`/Game/RoleSystem/Blueprints/RoleSystemRootComponent.BP_PsyonicalBlock` (`self.RoleSystemRootComponent`)))) (+ (`KismetMathLibrary.Conv_ByteToInt` (`self.EAgeStage`)) 1) 4) CoeffAgeStage))))

(fn `CalcUpperLimitParameters`
  (params (_LowerLimitParameters :type Integer) (CoeffUpperLimits :type "Float (double-precision)"))
  (returns (UpperLimitParameters :type Integer))
  (locals (LowerLimitParameters :type Integer))
  (bind _output_get (set `local.LowerLimitParameters` _LowerLimitParameters))
  (return (+ _output_get (`KismetMathLibrary.Round` (* _output_get CoeffUpperLimits)))))

(fn `IncreaseStage`
  (bind _output_get (set `self.EAgeStage` (cast `/Game/RoleSystem/Blueprints/AgeStages/EAgeStages` (+ (`self.EAgeStage`) 1))))
  (if (> _output_get (`self.EMaxAgeStage`))
    (set `self.EAgeStage` (`self.EMaxAgeStage`)))
  (return))

(fn `UserConstructionScript`)