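; BP_RoleSystemParent is a role system base Blueprint that provides a deferred begin-play mechanism, gated on references being ready.
; StartBeginPlayTimer sets a looping timer that retries BeforeBeginPlay until CheckReferences passes, then runs DoBeginPlay and clears the timer.
; CheckReferences returns true by default, while DoBeginPlay and AssignDelegates are empty hooks.
; Nothing in this Blueprint itself starts the timer.
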(event `AssignDelegates`)

(fn `BeforeBeginPlay`
  (if (`self.CheckReferences`)
    (`self.DoBeginPlay`)
    (`KismetSystemLibrary.K2_ClearAndInvalidateTimerHandle` (`self.BeginPlayTimer`))
    (return)
    (else
      (return))))

(fn `CheckReferences`
  (returns (IsValid :type Boolean))
  (return true))

(fn `DoBeginPlay`)

(fn `StartBeginPlayTimer`
  (bind _returnvalue (`KismetSystemLibrary.K2_SetTimer` null "BeforeBeginPlay" (`self.BeginPlayDeltaTime`) true))
  (set `self.BeginPlayTimer` _returnvalue))

(fn `UserConstructionScript`)