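; BP_RoleSystemItemsManager is the role system's manager for item effects on character stamina.
; It clamps incoming percentage deltas for jump stamina drain and stamina recovery rate to between -1 and 1, then writes them into BPStamina's item modifier variables.
; Startup runs through the parent's BeginPlay timer, with the reference check extended to require a valid BPStamina on the root component before caching it.
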(event `self.ReceiveBeginPlay`
  (`self.StartBeginPlayTimer`))

(fn `CheckReferences`
  (returns (IsValid :type Boolean))
  (return (and (`parent.CheckReferences`) (`KismetSystemLibrary.IsValid` (`/Game/RoleSystem/Blueprints/RoleSystemRootComponent.BP_Stamina` (`self.RoleSystemRootComponent`))))))

(fn `DoBeginPlay`
  (`parent.DoBeginPlay`)
  (set `self.BP_Stamina` (`/Game/RoleSystem/Blueprints/RoleSystemRootComponent.BP_Stamina` (`self.RoleSystemRootComponent`))))

(fn `DrainJumpStamina`
  (params (PrcDeltaDrainJumpStamina :type "Float (double-precision)"))
  (set `/Game/RoleSystem/Blueprints/SecondaryParameters/BP_Stamina.PrcDrainJumpStaminaItem` (`KismetMathLibrary.FClamp` PrcDeltaDrainJumpStamina -1.0) (`self.BP_Stamina`))
  (return))

(fn `RecoveryRaitStamina`
  (params (PrcDeltaRecoveryRaitStamina :type "Float (double-precision)"))
  (set `/Game/RoleSystem/Blueprints/SecondaryParameters/BP_Stamina.PrcRecoveryRaitStaminaItem` (`KismetMathLibrary.FClamp` PrcDeltaRecoveryRaitStamina -1.0) (`self.BP_Stamina`))
  (return))

(fn `StartBeginPlayTimer`
  (`parent.StartBeginPlayTimer`))

(fn `UserConstructionScript`
  (`parent.UserConstructionScript`))