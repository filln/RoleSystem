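; BP_PhysicalBlock is the physical block among the role system's basic parameters, computing that parameter's display value.
; CalcDisplayValue adds the summand from CalcSummandBasicBlock to BaseValue, stores the sum in DisplayValue, then returns it filtered through CheckDisplayValue.
; CheckDisplayValue defers entirely to the parent implementation, and the event graph and construction script add no logic of their own.
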(fn `CalcDisplayValue`
  (returns (DisplayValue :type "Float (double-precision)"))
  (locals (_DisplayValue :type "Float (double-precision)" :default 0.0))
  (bind _output_get (set `local._DisplayValue` (+ (`self.BaseValue`) (`self.CalcSummandBasicBlock`))))
  (bind _outputdisplayvalue (`self.CheckDisplayValue` _output_get))
  (return _outputdisplayvalue))

(fn `CheckDisplayValue`
  (params (InputDisplayValue :type "Float (double-precision)"))
  (returns (OutputDisplayValue :type "Float (double-precision)"))
  (bind _outputdisplayvalue (`parent.CheckDisplayValue` InputDisplayValue))
  (return _outputdisplayvalue))

(fn `UserConstructionScript`
  (`parent.UserConstructionScript`))