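; Base Blueprint for a role-system basic parameter, with a stub display value presumably overridden by children.
; Real value is display value times an effectivity coefficient, which BPAgeStages reduces when the display value lies between its lower and upper limits, slowing growth.
; Widget manager events flag whether this parameter's block type is the lead block, which enables its basic-block summand.
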(event `self.ReceiveBeginPlay`
  (`parent.ReceiveBeginPlay`)
  (`self.StartBeginPlayTimer`))

(event `self.AssignDelegates`
  (`parent.AssignDelegates`)
  (add `/Game/RoleSystem/Blueprints/BP_RoleSystemWidgetManager.OnSetIsLeadBlock` (`/Game/RoleSystem/Blueprints/RoleSystemRootComponent.BP_RoleSystemWidgetManager` (`self.RoleSystemRootComponent`)) (delegate `OnSetIsLeadBlock_Event_0`)))

(event `OnSetIsLeadBlock_Event_0`
  (params (IsLeadBlock :type Boolean) (TypeOfBlock :type "/Game/RoleSystem/Blueprints/BasicParameters/ETypeBlock Enum" :default "NewEnumerator0"))
  (`self.SetIsLeadBlock` IsLeadBlock TypeOfBlock))

(fn `CalcCurrentDeltaParameters`
  (params (LowerLimitParameters :type Integer))
  (returns (CurrentDeltaParameters :type "Float (double-precision)"))
  (return (- (`self.CalcDisplayValue`) (`KismetMathLibrary.Conv_IntToDouble` LowerLimitParameters))))

(fn `CalcDisplayValue`
  (returns (DisplayValue :type "Float (double-precision)"))
  (return 0.0))

(fn `CalcEffectivityCoeff `
  (returns (`EffectivityCoeff ` :type "Float (double-precision)"))
  (locals (LowerLimitParameters :type Integer :default 0) (_DisplayValue :type Integer))
  (bind _lowerlimitparameters (`local.LowerLimitParameters`))
  (set `local.LowerLimitParameters` (`/Game/RoleSystem/Blueprints/AgeStages/BP_AgeStages.CalcLowerLimitParameters` (`/Game/RoleSystem/Blueprints/RoleSystemRootComponent.BP_AgeStages` (`self.RoleSystemRootComponent`))))
  (set `local._DisplayValue` (`KismetMathLibrary.FTrunc` (`self.CalcDisplayValue`)))
  ;[0 1 1] Проверить, находится ли отображаемая характеристика в пределах нижнего и верхнего порога. Если да, то выполнить расчет, который уменьшает рост реальной характеристики.
  (if (and (> (`local._DisplayValue`) (`local.LowerLimitParameters`)) (<= (`local._DisplayValue`) (`/Game/RoleSystem/Blueprints/AgeStages/BP_AgeStages.CalcUpperLimitParameters` (`/Game/RoleSystem/Blueprints/RoleSystemRootComponent.BP_AgeStages` (`self.RoleSystemRootComponent`)) (`local.LowerLimitParameters`))))
    (return (- (`self.BaseEffectivityCoeff `) (`/Game/RoleSystem/Blueprints/AgeStages/BP_AgeStages.CalcDecreaseBaseEffectivityCoeff ` (`/Game/RoleSystem/Blueprints/RoleSystemRootComponent.BP_AgeStages` (`self.RoleSystemRootComponent`)) (`self.CalcCurrentDeltaParameters` _lowerlimitparameters) _lowerlimitparameters)))
    (else
      (return (`self.BaseEffectivityCoeff `)))))

(fn `CalcRealValue`
  (returns (RealValue :type "Float (double-precision)"))
  (return (* (`self.CalcDisplayValue`) (`self.CalcEffectivityCoeff `))))

(fn `CalcSummandBasicBlock`
  (returns (SummandBasicBlock :type "Float (double-precision)"))
  (if (`self.isLeadBlock`)
    (return (`self.SummandBasicBlock`))
    (else
      (return 0.0))))

(fn `CheckReferences`
  (returns (IsValid :type Boolean))
  (return (and (`KismetSystemLibrary.IsValid` (`/Game/RoleSystem/Blueprints/RoleSystemRootComponent.BP_RoleSystemWidgetManager` (`self.RoleSystemRootComponent`))) (`parent.CheckReferences`))))

(fn `DoBeginPlay`
  (`parent.DoBeginPlay`)
  (`self.AssignDelegates`))

(fn `SetIsLeadBlock`
  (params (IsLeadBlock :type Boolean) (TypeOfBlock :type "/Game/RoleSystem/Blueprints/BasicParameters/ETypeBlock Enum" :default "NewEnumerator0"))
  (if IsLeadBlock
    (if (`|EnumEquality` TypeOfBlock (`self.ETypeBlock`))
      (set `self.isLeadBlock` true)
      (else
        (set `self.isLeadBlock` false)))
    (else
      (set `self.isLeadBlock` false)))
  (return))

(fn `StartBeginPlayTimer`
  (`parent.StartBeginPlayTimer`))

(fn `UserConstructionScript`)