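; Blueprint function library for the RoleSystem that provides shortcut getters for core player references.
; GetHUD and GetPlayerController cast player 0's HUD and controller to their RoleSystem Blueprint classes, returning the typed reference with a success flag.
; Debug strings print when either cast fails and when the HUD cast succeeds.
; GetPlayerCharacter is an empty stub.
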(fn `GetHUD`
  (returns (`AsBP HUDRole System` :type "/Game/RoleSystem/Blueprints/CoreClasses/BP_HUDRoleSystem Object Reference") (`isCastSuccess?` :type Boolean))
  (bind _asbp_hudrole_system (cast `/Game/RoleSystem/Blueprints/CoreClasses/BP_HUDRoleSystem` (`PlayerController.GetHUD` (`GameplayStatics.GetPlayerController` null)))
    (:`then`
      (`KismetSystemLibrary.PrintString` null "GetHUD succsess")
      (return _asbp_hudrole_system true))
    (:`CastFailed`
      (`KismetSystemLibrary.PrintString` null "GetHUD failed")
      (return null false))))

(fn `GetPlayerCharacter`)

(fn `GetPlayerController`
  (returns (`AsBP Player Controller Role System` :type "/Game/RoleSystem/Blueprints/CoreClasses/BP_PlayerControllerRoleSystem Object Reference") (`isCastSuccess?` :type Boolean))
  (bind _asbp_player_controller_role_system (cast `/Game/RoleSystem/Blueprints/CoreClasses/BP_PlayerControllerRoleSystem` (`GameplayStatics.GetPlayerController` null))
    (:`then`
      (return _asbp_player_controller_role_system true))
    (:`CastFailed`
      (`KismetSystemLibrary.PrintString` null "GetPlayerController failed")
      (return null false))))