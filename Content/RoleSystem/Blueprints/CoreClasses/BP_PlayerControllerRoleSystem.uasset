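; Player controller for the Role System that manages input modes and game pausing.
; On BeginPlay it retries every 0.2 seconds until it gets and caches the Role System HUD.
; SetInputMode maps an enum to UI-only, game-only or game-and-UI input with matching cursor visibility.
; PauseOrUnpauseGame toggles pause only on state change, applies the given input mode and shows or hides an optional widget through the HUD.
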(event `self.ReceiveBeginPlay`
  (bind (_asbp_hudrole_system _iscastsuccess_) (`/Game/RoleSystem/Blueprints/CoreClasses/BPFL_ReferenceAggregator.GetHUD` :!label _label))
  (if _iscastsuccess_
    (set `self.BP_HUDRoleSystem` _asbp_hudrole_system)
    (else
      (`KismetSystemLibrary.Delay` 0.2)
      (goto _label))))

(fn `PauseOrUnpauseGame`
  (params (`isPause?` :type Boolean) (_OnWidgetIfPause :type "UserWidget Object Reference") (ZOrderOnWidget :type Integer) (_OffWidgetIfUnpause :type "UserWidget Object Reference") (InputModePause :type "/Game/RoleSystem/Enums/EInputMode Enum" :default "NewEnumerator0") (InputModeUnPause :type "/Game/RoleSystem/Enums/EInputMode Enum" :default "NewEnumerator0"))
  (if `isPause?`
    (if (`GameplayStatics.IsGamePaused`)
      (return)
      (else
        (`GameplayStatics.SetGamePaused` true)
        (if (`KismetSystemLibrary.IsValid` _OnWidgetIfPause)
          (`/Game/RoleSystem/Blueprints/CoreClasses/BP_HUDRoleSystem.ShowOrHideWidget` (`self.BP_HUDRoleSystem`) true _OnWidgetIfPause ZOrderOnWidget))
        (`self.SetInputMode` InputModePause)
        (return)))
    (elif (`GameplayStatics.IsGamePaused`)
      (`GameplayStatics.SetGamePaused` false)
      (`self.SetInputMode` InputModeUnPause)
      (if (`KismetSystemLibrary.IsValid` _OffWidgetIfUnpause)
        (`/Game/RoleSystem/Blueprints/CoreClasses/BP_HUDRoleSystem.ShowOrHideWidget` (`self.BP_HUDRoleSystem`) false _OffWidgetIfUnpause 0))
      (return)
      (else
        (return)))))

(fn `SetInputMode`
  (params (InputMode :type "/Game/RoleSystem/Enums/EInputMode Enum" :default "NewEnumerator0"))
  (if (`|EnumEquality` InputMode "NewEnumerator0")
    (set `self.bShowMouseCursor` true)
    (`WidgetBlueprintLibrary.SetInputMode_UIOnlyEx` null null)
    (elif (`|EnumEquality` InputMode "NewEnumerator1")
      (set `self.bShowMouseCursor` false)
      (`WidgetBlueprintLibrary.SetInputMode_GameOnly` null)
      (elif (`|EnumEquality` InputMode "NewEnumerator2")
        (set `self.bShowMouseCursor` true)
        (`WidgetBlueprintLibrary.SetInputMode_GameAndUIEx` null null "DoNotLock" false)
        (else
          (return)))))
  (return))

(fn `UserConstructionScript`)